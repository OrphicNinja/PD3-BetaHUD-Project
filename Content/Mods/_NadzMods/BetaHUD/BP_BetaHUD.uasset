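; BP_BetaHUD is a mod actor that restyles the existing in-game HUD.
; Each Tick searches for any HUD widget not yet cached, edits it, then stores the reference.
; It strips crew and player icons, hides the dodge bar, and shifts the pager and heist state by render translation.
; BeginPlay also creates a sub-objective blur widget, which is stored but not displayed here.
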(event `self.ReceiveBeginPlay`
  (bind _returnvalue (`|CreateWidget` "/Game/Mods/_NadzMods/BetaHUD/WBP_SubObjective_Blur.WBP_SubObjective_Blur_C"))
  (set `self.Blur` _returnvalue))

(event `self.ReceiveTick`
  (params (DeltaSeconds :type "Float (single-precision)"))
  (`parent.ReceiveTick` DeltaSeconds)
  (`|ExecutionSequence`
    (:`then_0`
      (if (== (`KismetArrayLibrary.Array_Length` (`self.PartyAICrew`)) 0)
        (bind _foundwidgets (`WidgetBlueprintLibrary.GetAllWidgetsOfClass` "/Game/UI/Widgets/HUD/PlayerAndParty/WBP_UI_Widget_PartyAICrewWidget.WBP_UI_Widget_PartyAICrewWidget_C" false))
        (for _array_element _foundwidgets
          (`Widget.RemoveFromParent` (`/Game/UI/Widgets/HUD/PlayerAndParty/WBP_UI_Widget_PartyAICrewWidget.Background` _array_element))
          (`Widget.RemoveFromParent` (`/Game/UI/Widgets/HUD/PlayerAndParty/WBP_UI_Widget_PartyAICrewWidget.Image_AICrewIcon_ERROR_DUPLICATE_0` _array_element))
          (`Widget.RemoveFromParent` (`PD3HUDAICrewStatusWidget.Image_AICrewIcon` _array_element))
          (`Widget.SetVisibility` (`/Game/UI/Widgets/HUD/PlayerAndParty/WBP_UI_Widget_PartyAICrewWidget.Image_AICrewIcon_ERROR_DUPLICATE_0` _array_element) "Collapsed")
          (`Widget.SetVisibility` (`/Game/UI/Widgets/HUD/PlayerAndParty/WBP_UI_Widget_PartyAICrewWidget.Background` _array_element) "Collapsed")
          (`Widget.SetVisibility` (`PD3HUDAICrewStatusWidget.Image_AICrewIcon` _array_element) "Collapsed")
          (`KismetArrayLibrary.Array_Add` (`self.PartyAICrew`) _array_element))))
    (:`then_1`
      (`self.LocalPlayerStatus`
        (:`then`)
        (:`else`
          (bind _foundwidgets_2 (`WidgetBlueprintLibrary.GetAllWidgetsOfClass` "/Game/UI/Widgets/HUD/PlayerAndParty/WBP_UI_Widget_PlayerStatusWidget.WBP_UI_Widget_PlayerStatusWidget_C" false))
          (for _array_element_2 _foundwidgets_2
            (bind _image_playericonbackground (`/Game/UI/Widgets/HUD/PlayerAndParty/WBP_UI_Widget_PlayerStatusWidget.Image_PlayerIconBackground` _array_element_2))
            (`Widget.SetVisibility` _image_playericonbackground "Collapsed")
            (`Widget.SetVisibility` (`/Game/UI/Widgets/HUD/PlayerAndParty/WBP_UI_Widget_PlayerStatusWidget.Image_PlayerIcon_ERROR_DUPLICATE_0` _array_element_2) "Collapsed")
            (`Widget.SetVisibility` (`PD3HUDPlayerStatusWidget.Image_PlayerIcon` _array_element_2) "Collapsed")
            (`Widget.RemoveFromParent` _image_playericonbackground)
            (`Widget.RemoveFromParent` (`/Game/UI/Widgets/HUD/PlayerAndParty/WBP_UI_Widget_PlayerStatusWidget.Image_PlayerIcon_ERROR_DUPLICATE_0` _array_element_2))
            (set `self.LocalPlayerStatus` _array_element_2)))))
    (:`then_2`
      (`self.DodgeBar`
        (:`then`)
        (:`else`
          (bind _foundwidgets_3 (`WidgetBlueprintLibrary.GetAllWidgetsOfClass` "/Game/UI/Widgets/HUD/PlayerAndParty/WBP_UI_Widget_AttributeBar.WBP_UI_Widget_AttributeBar_C" false))
          (for _array_element_3 _foundwidgets_3
            (if (`KismetStringLibrary.Contains` (`KismetSystemLibrary.GetObjectName` _array_element_3) "dodge")
              (`Widget.SetVisibility` _array_element_3 "Collapsed")
              (set `self.DodgeBar` _array_element_3))))))
    (:`then_3`
      (`self.Pager`
        (:`then`)
        (:`else`
          (bind _foundwidgets_4 (`WidgetBlueprintLibrary.GetAllWidgetsOfClass` "/Game/UI/Widgets/HUD/PlayerAndParty/WBP_UI_PagerWidget.WBP_UI_PagerWidget_C" false))
          (for _array_element_4 _foundwidgets_4
            (`Widget.SetRenderTranslation` _array_element_4 (`KismetMathLibrary.MakeVector2D` (- 40.0 292.245941) (- 605.0 65.0)))
            (set `self.Pager` _array_element_4)))))
    (:`then_4`
      (`self.HeistState`
        (:`then`)
        (:`else`
          (bind _foundwidgets_5 (`WidgetBlueprintLibrary.GetAllWidgetsOfClass` "/Game/UI/Widgets/HUD/WBP_UI_Widget_HeistState.WBP_UI_Widget_HeistState_C" false))
          (for _array_element_5 _foundwidgets_5
            (`Widget.SetRenderTranslation` _array_element_5 (`KismetMathLibrary.MakeVector2D` (- 200.0 960.0) (- 30.0 100.0)))
            (set `self.HeistState` _array_element_5)))))))

(fn `UserConstructionScript`)